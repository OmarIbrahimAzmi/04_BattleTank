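; Player-controllable tank Blueprint that drives, aims a camera rig and fires projectiles.
; Construction assigns meshes, the projectile class and track physics materials with collision notifications; BeginPlay wires barrel, turret and tracks into TankAiming and TankMovement.
; Move, turn and fire input forward to those components, while aim axes rotate the azimuth gimbal and spring arm separately, scaled by delta time.
; The health bar widget receives a reference to its owning tank.
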(event EventBeginPlay
  (Class|TankAimingComponent|Initialise (Variables|Default|GetTankAiming) (Variables|Default|GetTankBarrel) (Variables|Default|GetTurret))
  (Class|TankMovementComponent|Initialise (Variables|Default|GetTankMovement) (Variables|Default|GetLeftTrack) (Variables|Default|GetRightTrack))
  (CallFunction|IntialiseHealthBarWidget))

(event Input|ActionEvents|InputActionFire
  (params (Key :type Key%20Structure :default "None"))
  ;[1 1 1] Ballistic Input Binding
  (:Pressed
    (Class|TankAimingComponent|Fire (Variables|Default|GetTankAiming))))

(event Input|AxisEvents|InputAxisAimAzimuth
  (params (AxisValue :type Float%20%28single-precision%29))
  ;[1 1 1] Ballistic Input Binding
  (Transformation|AddLocalRotation (Variables|Default|GetAzimuth%20Gymbal) (Math|Rotator|MakeRotator 0.0 0.0 (* AxisValue (Utilities|Time|GetWorldDeltaSeconds) 1e+02)) false false))

(event Input|AxisEvents|InputAxisAimElevation
  (params (AxisValue :type Float%20%28single-precision%29))
  ;[1 1 1] Ballistic Input Binding
  (Transformation|AddLocalRotation (Variables|Default|GetSpringArm) (Math|Rotator|MakeRotator 0.0 (* AxisValue (Utilities|Time|GetWorldDeltaSeconds) 1e+02) 0.0) false false))

(event Input|AxisEvents|InputAxisTurnRight
  (params (AxisValue :type Float%20%28single-precision%29))
  ;[1 1 1] Movement Input Binding
  (Class|TankMovementComponent|IntendTurnRight (Variables|Default|GetTankMovement) AxisValue))

(event Input|AxisEvents|InputAxisMoveForward
  (params (AxisValue :type Float%20%28single-precision%29))
  ;[1 1 1] Movement Input Binding
  (Class|TankMovementComponent|IntendMoveForward (Variables|Default|GetTankMovement) AxisValue))

(fn ConstructionScript
  (bind _lefttrack (Variables|Default|GetLeftTrack))
  (bind _righttrack (Variables|Default|GetRightTrack))
  (Components|StaticMesh|SetStaticMesh (Variables|Default|GetTurret) "/Game/Tank/tank_fbx_Turret.tank_fbx_Turret")
  (Components|StaticMesh|SetStaticMesh (Variables|Default|GetTankBarrel) "/Game/Tank/tank_fbx_Barrel.tank_fbx_Barrel")
  (Variables|/Script/BattleTank.TankAimingComponent|SetProjectileBlueprint (Variables|Default|GetTankAiming) "/Game/Projectile/Projectile_BP.Projectile_BP_C")
  (Components|StaticMesh|SetStaticMesh _lefttrack "/Game/Tank/tank_fbx_Track.tank_fbx_Track")
  (Class|PrimitiveComponent|SetPhysMaterialOverride _lefttrack "/Game/Tank/Track.Track")
  (Class|PrimitiveComponent|SetNotifyRigidBodyCollision _lefttrack true)
  (Components|StaticMesh|SetStaticMesh _righttrack "/Game/Tank/tank_fbx_Track.tank_fbx_Track")
  (Class|PrimitiveComponent|SetPhysMaterialOverride _righttrack "/Game/Tank/Track.Track")
  (Class|PrimitiveComponent|SetNotifyRigidBodyCollision _righttrack true))

(fn IntialiseHealthBarWidget
  (bind _ashealth_bar_bp (Utilities|Casting|CastToHealthBar_BP (UserInterface|GetUserWidgetObject (Variables|Default|GetHealthBar)))
    (:then
      (Variables|/Game/Blueprints/UI/HealthBar_BP.HealthBar_BP_C|SetMyTank _ashealth_bar_bp self))
    (:CastFailed
      _))
  (return))